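; BP_Geyser is a water geyser hazard that periodically erupts and launches the third-person character straight up.
; Latent Delays on Tick form the repeating timer, starting an eruption about every five seconds and ending it three seconds later.
; Each eruption toggles the Niagara effect, an IsActive flag and the Box collision together.
; Box begin-overlap checks that flag before calling LaunchCharacter with a velocity override.
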(event `self.ReceiveTick`
  (params (DeltaSeconds :type "Float (single-precision)"))
  (`KismetSystemLibrary.Delay` 5.0)
  (`ActorComponent.Activate` (`self.Niagara`) false)
  (set `self.IsActive?` true)
  (`PrimitiveComponent.SetCollisionEnabled` (`self.Box`) "QueryAndPhysics")
  (`KismetSystemLibrary.Delay` 3.0)
  (`ActorComponent.Deactivate` (`self.Niagara`))
  (set `self.IsActive?` false)
  (`PrimitiveComponent.SetCollisionEnabled` (`self.Box`) "NoCollision"))

(event `self.Box.OnComponentBeginOverlap`
  (params (OverlappedComponent :type "PrimitiveComponent Object Reference") (OtherActor :type "Actor Object Reference") (OtherComp :type "PrimitiveComponent Object Reference") (OtherBodyIndex :type Integer) (bFromSweep :type Boolean) (SweepResult :type "HitResult Structure (by ref)"))
  (bind _asbp_third_person_character (cast `/Game/ThirdPerson/Blueprints/BP_ThirdPersonCharacter` OtherActor))
  (if (`self.IsActive?`)
    (`Character.LaunchCharacter` _asbp_third_person_character (0.0 0.0 2000.0) true true)))

(fn `UserConstructionScript`)